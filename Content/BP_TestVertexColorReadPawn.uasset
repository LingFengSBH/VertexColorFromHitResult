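; Test pawn that reads and displays the vertex color of the surface under the mouse cursor.
; It shows the cursor on begin play, then each tick deprojects the mouse position and runs a complex visibility line trace with debug drawing.
; The trace end is the scaled ray direction without the start offset.
; VertexColorFromHitResult extracts the color from the hit, which is printed on screen in that color when valid.
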(event EventBeginPlay
  (Variables|/Script/Engine.PlayerController|SetbShowMouseCursor (Game|GetPlayerController 0) true))

(event EventTick
  (params (DeltaSeconds :type Float%20%28single-precision%29))
  (bind _returnvalue (Class|WidgetLayoutLibrary|GetMousePositiononPlatform))
  (bind _outhit (Collision|LineTraceByChannel (.WorldPosition (Class|GameplayStatics|DeprojectScreentoWorld (Game|GetPlayerController 0) _returnvalue)) (* (.WorldDirection (Class|GameplayStatics|DeprojectScreentoWorld (Game|GetPlayerController 0) _returnvalue)) 5e+04) "TraceTypeQuery1" true 0 "ForOneFrame"))
  (bind (_outcolor _returnvalue_2) (Class|VertexColorfromHitResultBPLibrary|VertexColorfromHitResult _outhit))
  (if _returnvalue_2
    (Development|PrintString (Utilities|String|ToString(Integer) _outcolor) true true _outcolor)))

(fn ConstructionScript)